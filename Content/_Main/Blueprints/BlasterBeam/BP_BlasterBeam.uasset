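; BP_BlasterBeam is a blaster beam actor that reacts to impacts and ends the game when it hits its target pawn.
; On BeginPlay it binds the beam mesh's component hit event to a handler function.
; The handler spawns the NS_BeamBurst effect at the impact point, oriented along the surface normal.
; It then quits the game if the hit actor is TargetPawn, otherwise it destroys the beam.
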(event Custom|OnComponentHit_Event
  (params (HitComponent :type Primitive%20Component%20Object%20Reference) (OtherActor :type Actor%20Object%20Reference) (OtherComp :type Primitive%20Component%20Object%20Reference) (NormalImpulse :type Vector) (Hit :type Hit%20Result%20Structure%20%28by%20ref%29))
  (CallFunction|FHandleonHit OtherActor Hit))

(event EventBeginPlay
  (Collision|AssignOnComponentHit (Variables|Default|GetBeamMesh) (delegate Custom|OnComponentHit_Event)))

(fn ConstructionScript)

(fn FHandleonHit
  (params (HitActor :type Actor%20Object%20Reference) (Hit :type Hit%20Result%20Structure%20%28by%20ref%29))
  (bind (_bblockinghit _binitialoverlap _time _distance _location _impactpoint _normal) (Collision|BreakHitResult Hit))
  (Niagara|SpawnSystematLocation "/Game/_Main/_Assets/FX/NS_BeamBurst.NS_BeamBurst" _impactpoint (Math|Rotator|MakeRotfromX _normal))
  (if (== HitActor (Variables|Default|GetTargetPawn))
    (Game|QuitGame 0 "Quit" false)
    (else
      (Actor|DestroyActor))))