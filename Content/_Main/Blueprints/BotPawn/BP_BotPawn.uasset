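; Player-controlled flying bot pawn with mouse look, an overlay HUD, and health that quits the game on reaching zero.
; Enhanced Input drives FloatingPawnMovement along the control rotation's right, forward and up axes, while the mesh copies that rotation every tick.
; Firing alternates left and right rifle sockets via FlipFlop.
; A camera line trace sets the aim point, so each beam spawns at its socket angled toward it, with Niagara burst and sound.
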(event Input|EnhancedActionEvents|EnhancedInputActionIA_Fire
  (params (ActionValue :type Boolean) (ElapsedSeconds :type Float%20%28double-precision%29) (TriggeredSeconds :type Float%20%28double-precision%29) (InputAction :type Input%20Action%20Object%20Reference :default "/Game/_Main/Input/InputActions/IA_Fire.IA_Fire"))
  ;[1 0 1] Fire Rifle that Alternates betwen Rifle L and Rifle R
  (Utilities|FlowControl|FlipFlop
    (:A
      (CallFunction|FFireRilfe (Variables|Default|GetRifleSocketLeft)))
    (:B
      (CallFunction|FFireRilfe (Variables|Default|GetRifleSocketRight)))))

(event Input|EnhancedActionEvents|EnhancedInputActionIA_Look
  (params (ActionValue :type Vector%202D%20Structure) (ElapsedSeconds :type Float%20%28double-precision%29) (TriggeredSeconds :type Float%20%28double-precision%29) (InputAction :type Input%20Action%20Object%20Reference :default "/Game/_Main/Input/InputActions/IA_Look.IA_Look"))
  ;[1 0 1] Mouse Look using Mouse 2D Axis X/Y
  (Pawn|Input|AddControllerYawInput (.x ActionValue))
  (Pawn|Input|AddControllerPitchInput (.y ActionValue)))

(event Input|EnhancedActionEvents|EnhancedInputActionIA_Move
  (params (ActionValue :type Vector :default "0, 0, 0") (ElapsedSeconds :type Float%20%28double-precision%29) (TriggeredSeconds :type Float%20%28double-precision%29) (InputAction :type Input%20Action%20Object%20Reference :default "/Game/_Main/Input/InputActions/IA_Move.IA_Move"))
  ;[1 0 1] Movement using WASD. Also, Spacebar will Raise the Bot on the Z Axis.
  (CallFunction|FXAxisMovementInput (.x ActionValue))
  (CallFunction|FYAxisMovementInput (.y ActionValue))
  (CallFunction|FZAxisMovementInput (.z ActionValue)))

(event EventBeginPlay
  ;[0 0 1] BeginPlay - Add overlay to viewport.
  (bind _asplayer_controller (Utilities|Casting|CastToPlayerController (Pawn|GetController)))
  (Input|AddMappingContext (PlayerController|LocalPlayerSubsystems|GetEnhancedInputLocalPlayerSubsystem _asplayer_controller) "/Game/_Main/Input/IMC_Bot.IMC_Bot" 0 "(bIgnoreAllPressedKeysUntilRelease=True,bForceImmediately=False,bNotifyUserSettings=False)")
  (CallFunction|FInitializeUIWidget))

(event EventTick
  (params (DeltaSeconds :type Float%20%28single-precision%29))
  ;[1 0 1] Rotates the Mesh With the Controller
  (CallFunction|FRotateMeshtoController))

(event EventGetHurt
  (params (Damage :type Float%20%28double-precision%29))
  (bind _output_get (Variables|Default|SetHealth (- (Variables|Default|GetHealth) Damage)))
  (Development|PrintString (Utilities|String|Append "Took Damage. Health: " (Utilities|String|ToString(Float) _output_get)))
  (if (<= (Variables|Default|GetHealth) 0.0)
    (Game|QuitGame 0 "Quit" false)))

(fn ConstructionScript)

(fn FFireRilfe
  (params (InSocketName :type Name))
  (bind (_starttrace _endtrace) (CallFunction|FGetTrace))
  (bind _output_get (LocalVariables|SetTraceEnd _endtrace))
  (bind _returnvalue (CallFunction|FRifleTrace _starttrace _output_get (LocalVariables|GetTraceEnd)))
  (LocalVariables|SetTraceEnd _returnvalue)
  (Game|SpawnActorfromClass "/Game/_Main/Blueprints/BlasterBeam/BP_PlayerBlasterBeam.BP_PlayerBlasterBeam_C" (CallFunction|FSpawnBlasterBeam InSocketName (LocalVariables|GetTraceEnd)) "Undefined" "MultiplyWithRoot" 0 0 0)
  (CallFunction|FSpawnEffects InSocketName))

(fn FXAxisMovementInput
  (params (XAxisInput :type Float%20%28double-precision%29))
  (Class|PawnMovementComponent|AddInputVector (Variables|Default|GetFloatingPawnMovement) (* XAxisInput (Math|Vector|GetRightVector (Pawn|GetControlRotation :!class /Script/Engine.Pawn))) false))

(fn FYAxisMovementInput
  (params (YAxisINput :type Float%20%28double-precision%29))
  (Class|PawnMovementComponent|AddInputVector (Variables|Default|GetFloatingPawnMovement) (* YAxisINput (Math|Vector|GetForwardVector (Pawn|GetControlRotation :!class /Script/Engine.Pawn))) false))

(fn FRotateMeshtoController
  (Transformation|SetWorldRotation (Variables|Default|GetBotMesh) (Pawn|GetControlRotation :!class /Script/Engine.Pawn) false false))

(fn FZAxisMovementInput
  (params (ZAxisInput :type Float%20%28double-precision%29))
  (Class|PawnMovementComponent|AddInputVector (Variables|Default|GetFloatingPawnMovement) (* ZAxisInput (Math|Vector|GetUpVector (Pawn|GetControlRotation :!class /Script/Engine.Pawn))) false))

(fn FInitializeUIWidget
  (bind _returnvalue (UserInterface|CreateWidget "/Game/_Main/Blueprints/UI/WBP_OverlayHUD.WBP_OverlayHUD_C"))
  (bind _output_get (Variables|Default|SetOVerlayHUD_REF _returnvalue))
  (UserInterface|Viewport|AddtoViewport _output_get 0))

(fn FGetTrace
  (bind _camera (Variables|Default|GetCamera))
  (bind _returnvalue (Transformation|GetWorldLocation _camera))
  (return _returnvalue (+ _returnvalue (* (Math|Vector|GetForwardVector _camera) (Variables|Combat|GetTraceDistance)))))

(fn FSpawnEffects
  (params (InSocketName :type Name))
  (bind _botmesh (Variables|Default|GetBotMesh))
  (bind _returnvalue (Transformation|GetSocketTransform _botmesh InSocketName "RTS_World"))
  (Niagara|SpawnSystematLocation "/Game/_Main/_Assets/FX/NS_BeamBurst.NS_BeamBurst" (.location _returnvalue) (.rotation _returnvalue))
  (Audio|PlaySoundatLocation "/Game/_Main/_Assets/Sounds/Drone/SFX_EnergyRifle.SFX_EnergyRifle" (.location _returnvalue) "0, 0, 0" 1.0 1.0 0.0 0 0 0 0))

(fn FSpawnBlasterBeam
  (params (InSocketName :type Name) (Target :type Vector%20%28by%20ref%29))
  (bind _botmesh (Variables|Default|GetBotMesh))
  (bind _returnvalue (Transformation|GetSocketTransform _botmesh InSocketName "RTS_World"))
  (return (Math|Transform|MakeTransform (.location _returnvalue) (Math|Rotator|FindLookatRotation (.location _returnvalue) Target))))

(fn FRifleTrace
  (params (StartTrace :type Vector) (EndTrace :type Vector) (TraceEnd :type Vector))
  (bind _outhit (Collision|LineTraceByChannel StartTrace EndTrace "TraceTypeQuery1" false 0 "None" true "(R=1.000000,G=0.000000,B=0.000000,A=1.000000)" "(R=0.000000,G=1.000000,B=0.000000,A=1.000000)" 6e+01))
  (return (Math|Vector|SelectVector (.ImpactPoint (Collision|BreakHitResult _outhit)) TraceEnd (.bBlockingHit (Collision|BreakHitResult _outhit)))))