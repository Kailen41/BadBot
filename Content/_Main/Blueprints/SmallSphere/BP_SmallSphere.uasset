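; Small sphere pickup for the BadBot game that drifts along, increments the game mode's score when a Pawn overlaps it, then disappears.
; Each tick moves it along its forward vector while a random spin set at BeginPlay rotates the actor, curving its path.
; Timelines scale the mesh to wink it in on spawn and out on overlap or lifetime expiry, destroying the actor when wink-out finishes.
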(event OnComponentBeginOverlap(SphereVolume)
  (params (OverlappedComponent :type Primitive%20Component%20Object%20Reference) (OtherActor :type Actor%20Object%20Reference) (OtherComp :type Primitive%20Component%20Object%20Reference) (OtherBodyIndex :type Integer) (bFromSweep :type Boolean) (SweepResult :type Hit%20Result%20Structure%20%28by%20ref%29))
  ;[1 0 1] Handle Overlap
  (if (Class|GameplayStatics|ObjectIsA OtherActor "/Script/Engine.Pawn")
    (bind _asbp_bad_bot_game_mode (Utilities|Casting|CastToBP_BadBotGameMode (Game|GetGameMode)))
    (Utilities|IsValid _asbp_bad_bot_game_mode
      (:Is%20Valid
        (Default|FIncrementScore _asbp_bad_bot_game_mode)
        (CallFunction|WinkOut)))))

(event Custom|WinkOut
  ;[0 0 1] BeginPlay
  ;;[1 0 1] Start WinkOut Timeline
  (if (not (Variables|Default|GetIsWinking?))
    (Variables|Default|SetIsWinking? true)
    (bind _scale_alpha (Timeline|WinkOut_TL Play)
      (:Update
        (CallFunction|FScaleSphere _scale_alpha))
      (:Finished
        (Actor|DestroyActor)))))

(event Custom|WinkIn
  ;[1 0 1] Wink into Existence
  (bind _scale_alpha (Timeline|WinkIn_TL Play)
    (:Update
      (Transformation|SetWorldScale3D (Variables|Default|GetSphereMesh) _scale_alpha))))

(event EventTick
  (params (DeltaSeconds :type Float%20%28single-precision%29))
  ;[1 0 1] Update Location and Rotation
  (CallFunction|FUpdateLocation DeltaSeconds)
  (CallFunction|FUpdateRotation DeltaSeconds))

(event EventBeginPlay
  ;[0 0 1] BeginPlay
  (CallFunction|Winkin)
  (CallFunction|FInitialzeDeltaRotation)
  ;;[1 0 1] Start WinkOut Timeline
  (Utilities|Time|SetTimerbyEvent (delegate Custom|WinkOut) (Variables|Default|GetLifeTime)))

(fn ConstructionScript)

(fn FInitialzeDeltaRotation
  (Variables|SphereMovement|SetDelta%20Rotation (* (Math|Random|RandomRotator false) (Variables|SphereMovement|GetRotationScaleFactor))))

(fn FUpdateLocation
  (params (DeltaSeconds :type Float%20%28double-precision%29))
  (Transformation|AddActorWorldOffset (* (* DeltaSeconds (Variables|SphereMovement|GetSpeed)) (Transformation|GetActorForwardVector))))

(fn FUpdateRotation
  (params (DeltaSeconds :type Float%20%28single-precision%29))
  (Class|Actor|AddActorWorldRotation (* (Variables|SphereMovement|GetDelta%20Rotation) DeltaSeconds)))

(fn FScaleSphere
  (params (Scale :type Float%20%28single-precision%29))
  (Transformation|SetWorldScale3D (Variables|Default|GetSphereMesh) (Math|Vector|MakeVector Scale Scale Scale)))